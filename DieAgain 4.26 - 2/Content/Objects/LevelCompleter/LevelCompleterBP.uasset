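; Level actor that sets the win condition, ends the level and owns time-dilation effects for game over, sniper hits and the slow-time power-up.
; BeginPlay waits briefly for enemies, counts them for Kill Them All and applies level lighting settings.
; Enemy deaths, VIP death or box overlap trigger completion; Survive has no logic here.
; Completion slows time, saves best score, unlocks and controlled-character stats, then opens the next level.
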(event `CleanTimeDilation`
  (params (ChameleonRef :type "/Game/Chameleon/Chameleon Object Reference"))
  (set `Actor.CustomTimeDilation` 1.0 (`GameplayStatics.GetPlayerPawn` 0))
  (`GameplayStatics.SetGlobalTimeDilation` 1.0)
  (if (`KismetSystemLibrary.IsValid` ChameleonRef)
    (set `/Game/Chameleon/Chameleon.Alcohol` false ChameleonRef)))

(event `GameOverSlowTime`
  (set `self.IsGameOver` true)
  (`self.CleanTimeDilation` null)
  (`GameplayStatics.SetGlobalTimeDilation` 0.33) ; Nota: Hacerlo con el LevelCompleter
  (`KismetSystemLibrary.Delay` 0.5)
  (if (not (`self.IsLevelCompleted`))
    (`GameplayStatics.SetGlobalTimeDilation` 0.0) ; Hacerlo con el LevelCompleter
  ))

(event `SniperHit`
  (if (not (`self.IsLevelCompleted`))
    (set `self.IsSniperHit` true)
    (`GameplayStatics.SetGlobalTimeDilation` 0.1)
    (`KismetSystemLibrary.Delay` 0.05)
    (`self.CleanTimeDilation` null)
    (set `self.IsSniperHit` false)))

(event `PowerUpSlowTime`
  (params (ChameleonRef :type "/Game/Chameleon/Chameleon Object Reference"))
  (if (not (and (and (`self.IsLevelCompleted`) (`self.IsGameOver`)) (`self.IsSniperHit`)))
    (`GameplayStatics.SetGlobalTimeDilation` 0.2)
    (set `Actor.CustomTimeDilation` 5.0 (`GameplayStatics.GetPlayerPawn` 0))
    (set `/Game/Chameleon/Chameleon.Alcohol` true ChameleonRef)
    (set `/Game/Chameleon/Chameleon.Alcohol Offset` 2.75 ChameleonRef)
    (`KismetSystemLibrary.Delay` 1.0)
    (if (not (and (and (`self.IsLevelCompleted`) (`self.IsGameOver`)) (`self.IsSniperHit`)))
      (`self.CleanTimeDilation` ChameleonRef))))

(event `Level_Completed`
  (bind _returnvalue (`GameplayStatics.GetPlayerCharacter` 0))
  (set `self.IsLevelCompleted` true)
  (`self.CleanTimeDilation` null)
  (`GameplayStatics.SetGlobalTimeDilation` 0.5)
  (bind _asmy_game_instance (cast `/Game/MyGameInstance/MyGameInstance` (`GameplayStatics.GetGameInstance`)))
  (set `/Game/MyGameInstance/MyGameInstance.IsLevelCompleted` true _asmy_game_instance)
  (`KismetSystemLibrary.Delay` 0.5)
  (`GameplayStatics.SetGlobalTimeDilation` 0.25)
  (`KismetSystemLibrary.Delay` 0.4)
  (`self.GetTotalPoints` (`self.LevelCompleted`))
  (`self.SetExtraAmmo`)
  (`self.SetPowerUpUnlocked`)
  (bind _asmy_game_instance_2 (cast `/Game/MyGameInstance/MyGameInstance` (`GameplayStatics.GetGameInstance`)))
  (`/Game/MyGameInstance/MyGameInstance.LevelUnlocked` _asmy_game_instance_2 (`self.UnlockedLevel`))
  (bind _asthird_person_character (cast `/Game/ThirdPersonBP/Blueprints/ThirdPersonCharacter` _returnvalue)
    (:`then`
      (if (`Pawn.IsPlayerControlled` _asthird_person_character)
        (bind _mesh (`Character.Mesh` _asthird_person_character))
        (`/Game/MyGameInstance/MyGameInstance.SavePlayerStats` _asmy_game_instance_2 (`/Game/ThirdPersonBP/Blueprints/ThirdPersonCharacter.WeaponEquiped` _asthird_person_character) (`/Game/ThirdPersonBP/Blueprints/ThirdPersonCharacter.Ammunition` _asthird_person_character) 0 (`SkinnedMeshComponent.SkeletalMesh` _mesh) (`PrimitiveComponent.GetMaterial` _mesh 0) (`PrimitiveComponent.GetMaterial` _mesh 1) false)
        (`GameplayStatics.OpenLevel` (`self.NameOfNextLevel`) :!label _label)
        (else
          (bind _asenemy_shooting_ch (cast `/Game/Enemies/EnemyShootingCh` _returnvalue :!label _label_2))
          (if (`Pawn.IsPlayerControlled` _asenemy_shooting_ch)
            (if (`/Game/Enemies/EnemyShootingCh.Exposed` _asenemy_shooting_ch)
              (bind _weapon (`/Game/Enemies/EnemyShootingCh.Weapon` _asenemy_shooting_ch))
              (bind _ammunition (`/Game/Enemies/EnemyShootingCh.Ammunition` _asenemy_shooting_ch))
              (bind _skeletalmesh (`/Game/Enemies/EnemyShootingCh.SkeletalMesh` _asenemy_shooting_ch))
              (bind _skeletalmesh_2 (`SkinnedMeshComponent.SkeletalMesh` _skeletalmesh))
              (bind _returnvalue_2 (`PrimitiveComponent.GetMaterial` _skeletalmesh 0))
              (bind _returnvalue_3 (`PrimitiveComponent.GetMaterial` _skeletalmesh 1))
              (bind _isslave (`/Game/Enemies/EnemyShootingCh.IsSlave` _asenemy_shooting_ch))
              (`/Game/MyGameInstance/MyGameInstance.SavePlayerStats` _asmy_game_instance_2 _weapon _ammunition (`/Game/Enemies/EnemyShootingCh.PreviousSquad` _asenemy_shooting_ch) _skeletalmesh_2 _returnvalue_2 _returnvalue_3 _isslave)
              (goto _label)
              (else
                (`/Game/MyGameInstance/MyGameInstance.SavePlayerStats` _asmy_game_instance_2 _weapon _ammunition (`/Game/Enemies/EnemyShootingCh.Squad` _asenemy_shooting_ch) _skeletalmesh_2 _returnvalue_2 _returnvalue_3 _isslave)
                (goto _label)))))))
    (:`CastFailed`
      (goto _label_2))))

(event `self.ReceiveTick`
  (params (DeltaSeconds :type "Float (single-precision)")))

(event `self.ReceiveBeginPlay`
  (`|ExecutionSequence`
    (:`then_0`
      (bind _asthird_person_character (cast `/Game/ThirdPersonBP/Blueprints/ThirdPersonCharacter` (`GameplayStatics.GetPlayerCharacter` 0)))
      (set `/Game/ThirdPersonBP/Blueprints/ThirdPersonCharacter.IsDark` (`self.IsDarkLevel`) _asthird_person_character))
    (:`then_1`
      (`KismetSystemLibrary.Delay` 0.1) ; Delay para que los enemigos puedan setearse. Sin esto, no funciona ningun metodo de superar el nivel de este actor
      (`|ExecutionSequence`
        (:`then_0`
          (switch `/Game/Objects/LevelCompleter/EnumTypeOfLevelCompleted` (`self.ConditionToWin`)
            (:`NewEnumerator0`
              (set `self.SetedConditionToWin` "NewEnumerator0")
              (set `self.EnemyActorsToEliminate` 0)
              (bind _outactors (`GameplayStatics.GetAllActorsOfClass` "/Game/Enemies/EnemyShootingCh.EnemyShootingCh_C"))
              (for _array_element _outactors
                (bind _asenemy_shooting_ch (cast `/Game/Enemies/EnemyShootingCh` _array_element))
                (if (not (`/Game/Enemies/EnemyShootingCh.IsSlave` _asenemy_shooting_ch))
                  (`/Engine/EditorBlueprintResources/StandardMacros.IncrementInt` (`self.EnemyActorsToEliminate`))))
              (bind _outactors_2 (`GameplayStatics.GetAllActorsOfClass` "/Game/Enemies/EnemyDogCh.EnemyDogCh_C"))
              (for _array_element_2 _outactors_2
                (bind _asenemy_dog_ch (cast `/Game/Enemies/EnemyDogCh` _array_element_2))
                (if (`KismetSystemLibrary.IsValid` _asenemy_dog_ch)
                  (`/Engine/EditorBlueprintResources/StandardMacros.IncrementInt` (`self.EnemyActorsToEliminate`)))))
            (:`NewEnumerator1`
              (set `self.SetedConditionToWin` "NewEnumerator1"))
            (:`NewEnumerator2`
              (set `self.SetedConditionToWin` "NewEnumerator2")
              (`SceneComponent.SetVisibility` (`self.Cube`) true false))
            (:`NewEnumerator3`
              (set `self.SetedConditionToWin` "NewEnumerator3"))))
        (:`then_1`
          (bind _outactors_3 (`GameplayStatics.GetAllActorsOfClass` "/Game/Enemies/EnemyShootingCh.EnemyShootingCh_C"))
          (for _array_element_3 _outactors_3
            (bind _asenemy_shooting_ch_2 (cast `/Game/Enemies/EnemyShootingCh` _array_element_3))
            (set `/Game/Enemies/EnemyShootingCh.IsDark` (`self.IsDarkLevel`) _asenemy_shooting_ch_2)
            (bind _asmy_game_instance (cast `/Game/MyGameInstance/MyGameInstance` (`GameplayStatics.GetGameInstance`)))
            (if (`/Game/MyGameInstance/MyGameInstance.NF_Enemies` _asmy_game_instance)
              (bind _spotlight (`/Game/Enemies/EnemyShootingCh.SpotLight` _asenemy_shooting_ch_2))
              (`SpotLightComponent.SetOuterConeAngle` _spotlight 30.0)
              (`SceneComponent.K2_SetRelativeLocation` _spotlight (+ (`SceneComponent.RelativeLocation` _spotlight) (0.0 0.0 -60.0)) false true)
              (bind _asthird_person_character_2 (cast `/Game/ThirdPersonBP/Blueprints/ThirdPersonCharacter` (`GameplayStatics.GetPlayerCharacter` 0)))
              (bind _spotlight_2 (`/Game/ThirdPersonBP/Blueprints/ThirdPersonCharacter.SpotLight` _asthird_person_character_2))
              (`SpotLightComponent.SetOuterConeAngle` _spotlight_2 30.0)
              (bind (_relativelocation_x _relativelocation_y) (`KismetMathLibrary.BreakVector` (`SceneComponent.RelativeLocation` _spotlight_2)))
              (`SceneComponent.K2_SetRelativeLocation` _spotlight_2 (`KismetMathLibrary.MakeVector` _relativelocation_x _relativelocation_y 30.387909) false true))))
        (:`then_2`
          (bind _outactors_4 (`GameplayStatics.GetAllActorsOfClass` "/Game/CameraActor/CameraActor.CameraActor_C"))
          (for _array_element_4 _outactors_4
            (bind _ascamera_actor (cast `/Game/CameraActor/CameraActor` _array_element_4))
            (set `self.CameraActor` _ascamera_actor)))))))

(event `self.BoxLevelCompleted.OnComponentBeginOverlap`
  (params (OverlappedComponent :type "PrimitiveComponent Object Reference") (OtherActor :type "Actor Object Reference") (OtherComp :type "PrimitiveComponent Object Reference") (OtherBodyIndex :type Integer) (bFromSweep :type Boolean) (SweepResult :type "HitResult Structure (by ref)"))
  (bind _returnvalue (`GameplayStatics.GetPlayerCharacter` 0))
  (if (`Controller.IsPlayerController` (`self.GetInstigatorController` OtherActor))
    (bind _asenemy_shooting_ch (cast `/Game/Enemies/EnemyShootingCh` _returnvalue)
      (:`then`
        (if (== OtherComp (`/Game/Enemies/EnemyShootingCh.BoxCollision` _asenemy_shooting_ch))
          (switch `/Game/Objects/LevelCompleter/EnumTypeOfLevelCompleted` (`self.SetedConditionToWin`) :!label _label_3
            (:`NewEnumerator2`
              (`self.Level_Completed`)))))
      (:`CastFailed`
        (bind _asthird_person_character (cast `/Game/ThirdPersonBP/Blueprints/ThirdPersonCharacter` _returnvalue))
        (if (== OtherComp (`/Game/ThirdPersonBP/Blueprints/ThirdPersonCharacter.BoxCollision` _asthird_person_character))
          (goto _label_3))))))

(fn `ComparationPuntuation`
  (params (StoredPuntuation :type Integer) (NewPuntuation :type Integer))
  (returns (MaxPuntuation :type Integer))
  (locals (MaximumPuntuation :type Integer))
  (`KismetSystemLibrary.PrintString` (`KismetStringLibrary.Concat_StrStr` "Stored" (`KismetStringLibrary.Conv_IntToString` StoredPuntuation)))
  (`KismetSystemLibrary.PrintString` (`KismetStringLibrary.Concat_StrStr` "New" (`KismetStringLibrary.Conv_IntToString` NewPuntuation)))
  (if (>= StoredPuntuation NewPuntuation)
    (set `local.MaximumPuntuation` StoredPuntuation)
    (else
      (set `local.MaximumPuntuation` NewPuntuation)))
  (return (`local.MaximumPuntuation`)))

(fn `EnemyDeath`
  (bind _enemyactorstoeliminate (`self.EnemyActorsToEliminate`))
  (switch `/Game/Objects/LevelCompleter/EnumTypeOfLevelCompleted` (`self.SetedConditionToWin`)
    (:`NewEnumerator0`
      (`/Engine/EditorBlueprintResources/StandardMacros.DecrementInt` _enemyactorstoeliminate
        (:`  `
          (if (<= _enemyactorstoeliminate 0)
            (`KismetSystemLibrary.PrintString` "All Enemies are Death")
            (`self.Level_Completed`)))))))

(fn `GetTotalPoints`
  (params (LevelCompleted :type "/Game/Enemies/EnumLevelsUnlockeds Enum" :default "NewEnumerator10"))
  (bind _returnvalue (`KismetMathLibrary.Conv_ByteToInt` LevelCompleted))
  (bind _asmy_game_instance (cast `/Game/MyGameInstance/MyGameInstance` (`GameplayStatics.GetGameInstance`)))
  (bind _output_get (set `/Game/MyGameInstance/MyGameInstance.LVPoints` (+ (* (`/Game/MyGameInstance/MyGameInstance.ComboMult` _asmy_game_instance) (`/Game/MyGameInstance/MyGameInstance.CurrentPoints` _asmy_game_instance)) (`/Game/MyGameInstance/MyGameInstance.LVPoints` _asmy_game_instance)) _asmy_game_instance))
  (set `/Game/MyGameInstance/MyGameInstance.ComboMult` 0 _asmy_game_instance)
  (set `/Game/MyGameInstance/MyGameInstance.CurrentPoints` 0 _asmy_game_instance)
  (bind _returnvalue_2 (`GameplayStatics.LoadGameFromSlot` "Save_File"))
  (bind _assave_game_bp (cast `/Game/SaveGame/SaveGameBP` _returnvalue_2))
  (bind _puntuationlevels (`/Game/SaveGame/SaveGameBP.PuntuationLevels` _assave_game_bp))
  (bind _maxpuntuation (`self.ComparationPuntuation` (`|GetArrayItem` _puntuationlevels _returnvalue) _output_get))
  (`KismetArrayLibrary.Array_Set` _puntuationlevels _returnvalue _maxpuntuation)
  (`GameplayStatics.SaveGameToSlot` _assave_game_bp "Save_File"))

(fn `PowerUpSlowDownTimeOLD`
  (if (`self.IsLevelCompleted`)
    _
    (elif (not (`self.IsGameOver`))
      (`GameplayStatics.SetGlobalTimeDilation` 0.2)
      (set `Actor.CustomTimeDilation` 5.0 (`GameplayStatics.GetPlayerPawn` 0)))))

(fn `SetExtraAmmo`
  (if (`self.ExtraAmmoRifle`)
    (bind _returnvalue (`GameplayStatics.LoadGameFromSlot` "Save_File"))
    (bind _assave_game_bp (cast `/Game/SaveGame/SaveGameBP` _returnvalue))
    (set `/Game/SaveGame/SaveGameBP.ExtraAmmoRifle` true _assave_game_bp)
    (`GameplayStatics.SaveGameToSlot` _returnvalue "Save_File")
    (elif (`self.ExtraAmmoShotgun`)
      (bind _returnvalue_2 (`GameplayStatics.LoadGameFromSlot` "Save_File"))
      (bind _assave_game_bp_2 (cast `/Game/SaveGame/SaveGameBP` _returnvalue_2))
      (set `/Game/SaveGame/SaveGameBP.ExtraAmmoShotgun` true _assave_game_bp_2)
      (`GameplayStatics.SaveGameToSlot` _returnvalue_2 "Save_File"))))

(fn `SetPowerUpUnlocked`
  (if (`self.IsPowerUpUnlock`)
    (bind _returnvalue (`GameplayStatics.LoadGameFromSlot` "Save_File"))
    (bind _assave_game_bp (cast `/Game/SaveGame/SaveGameBP` _returnvalue))
    (set `/Game/SaveGame/SaveGameBP.PowerUpUnlocked` true _assave_game_bp)
    (`GameplayStatics.SaveGameToSlot` _returnvalue "Save_File")))

(fn `UserConstructionScript`)

(fn `VIPEliminated`
  (switch `/Game/Objects/LevelCompleter/EnumTypeOfLevelCompleted` (`self.SetedConditionToWin`)
    (:`NewEnumerator1`
      (`KismetSystemLibrary.PrintString` "VIPDeath")
      (`self.Level_Completed`))))

(fn `WinConditionReached`)